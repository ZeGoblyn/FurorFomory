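; Sergeant enemy NPC with a timed melee fist attack, a player-spotted sound and ragdoll death.
; MeleeAttack sets attack state and opens a delayed damage window, during which fist overlaps subtract player health unless parrying.
; Tick watches health and, once depleted, ragdolls the body, deactivates the Blackboard and calls a random pickup drop gated by Mort.
; Random patrol, hit reaction and AI perception logic are disconnected.
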(event OnComponentBeginOverlap(Fist_box)
  (params (OverlappedComponent :type Primitive%20Component%20Object%20Reference) (OtherActor :type Actor%20Object%20Reference) (OtherComp :type Primitive%20Component%20Object%20Reference) (OtherBodyIndex :type Integer) (bFromSweep :type Boolean) (SweepResult :type Hit%20Result%20Structure%20%28by%20ref%29))
  ;[1 1 1] ApplyDamage
  (Utilities|IsValid OtherActor
    (:Is%20Valid
      (if (and (Variables|Default|GetSergentDamage) (not (Math|Boolean|ORBoolean (Variables|/Game/FirstPersonBP/Blueprints/FirstPersonCharacter.FirstPersonCharacter_C|GetSword_Parry (stale _asfirst_person_character)) (Variables|/Game/FirstPersonBP/Blueprints/FirstPersonCharacter.FirstPersonCharacter_C|GetLance_Parry (stale _asfirst_person_character)) (Variables|/Game/FirstPersonBP/Blueprints/FirstPersonCharacter.FirstPersonCharacter_C|GetHammer_Parry (stale _asfirst_person_character)))))
        (bind _asfirst_person_character (Utilities|Casting|CastToFirstPersonCharacter OtherActor))
        (Audio|PlaySoundatLocation "/Game/FirstPersonBP/Blueprints/HeavyWound.HeavyWound" (Transformation|GetActorLocation) "0, 0, 0" 1.0 1.0 0.0 0 0 _asfirst_person_character)
        (Variables|/Game/FirstPersonBP/Blueprints/FirstPersonCharacter.FirstPersonCharacter_C|SetPV _asfirst_person_character (- (Variables|/Game/FirstPersonBP/Blueprints/FirstPersonCharacter.FirstPersonCharacter_C|GetPV _asfirst_person_character) (Variables|Default|GetSergentFistDamage)))))))

(event OnTargetPerceptionUpdated(AIPerception)
  (params (Actor :type Actor%20Object%20Reference) (Stimulus :type AI%20Stimulus%20Structure))
  ;[1 1 1] Navigation et patrouille (hors service)
)

(event OnSeePawn(PawnSensing)
  (params (Pawn :type Pawn%20Object%20Reference))
  ;[1 1 1] Son de détection joueur
  (if (Variables|Default|GetSergentVivant)
    (Utilities|Casting|CastToFirstPersonCharacter Pawn)
    (Utilities|FlowControl|Sequence
      (:then_0
        (Utilities|FlowControl|DoOnce false :!label _label
          (:Completed
            (Audio|PlaySoundatLocation "/Game/Ennemies/NPC/Sergent_2/Sergent_spot.Sergent_spot" (Transformation|GetActorLocation) "0, 0, 0" 1.0 1.0 0.0 0 0 0))))
      (:then_1
        (Utilities|FlowControl|RetriggerableDelay 2.0)
        (goto _label Reset)))))

(event OnComponentBeginOverlap(Mesh)
  (params (OverlappedComponent :type Primitive%20Component%20Object%20Reference) (OtherActor :type Actor%20Object%20Reference) (OtherComp :type Primitive%20Component%20Object%20Reference) (OtherBodyIndex :type Integer) (bFromSweep :type Boolean) (SweepResult :type Hit%20Result%20Structure%20%28by%20ref%29)))

(event Custom|MoveNPC
  ;[1 1 1] Navigation et patrouille (hors service)
  ;;[1 1 1] Déplacement aléatoire sur NavMesh
)

(event Custom|Hit
  ;[1 1 1] Tentative animation blessure
)

(event Custom|deathDrop
  ;[1 1 1] Methode drop de ressources
  (if (Variables|Default|Getmort)
    (Game|SpawnActorfromClass (Utilities|Select :Index (Math|Random|RandomInteger 6) :Option%200 "/Game/sA_PickupSet_1/COLLEC_regen.COLLEC_regen_C" :Option%201 "/Game/sA_PickupSet_1/COLLEC_adren.COLLEC_adren_C") (Math|Conversions|ToTransform(Vector) (Transformation|GetActorLocation)) "Undefined" 0 0)))

(event Custom|DamageActivation
  ;[1 1 1] Activation des Dégats pendant l'animation d'attaque
  (Utilities|FlowControl|Delay 0.6)
  (Variables|Default|SetSergentDamage true)
  (Utilities|FlowControl|Delay 0.82)
  (Variables|Default|SetSergentDamage false))

(event EventBeginPlay
  ;[1 1 1] Init PV et Identification d'armes
  (bind _asbp_epee (Utilities|Casting|CastToBP_EPEE (Components|GetOwner)))
  (Variables|Default|SetAs%20BP%20EPEE _asbp_epee)
  (Variables|Default|Setn_pvMAX_grunt (Variables|Default|Getn_pv)))

(event Collision|EventActorBeginOverlap
  (params (OtherActor :type Actor%20Object%20Reference))
  ;[1 1 1] Navigation et patrouille (hors service)
)

(event EventGruntHit
  ;[1 1 1] Tentative animation blessure
)

(event EventTick
  (params (DeltaSeconds :type Float%20%28single-precision%29))
  ;[1 1 1] Etat de santé et de mort
  (if (<= (Variables|Default|Getn_pv) 0.0)
    (Variables|Default|SetSergentVivant false)
    (Utilities|FlowControl|DoOnce false
      (:Completed
        (CallFunction|DeathRagdoll)
        ;[1 1 1] Drop ressources
        (CallFunction|DeathDrop)))))

(event EventMeleeAttack
  ;[1 1 1] Animation d'attaque
  (if (Variables|Default|GetSergentVivant)
    (Development|PrintString "ATTACK" true true "(R=1.000000,G=0.000000,B=0.000000,A=1.000000)")
    (Variables|Default|SetSergentAttack true)
    (CallFunction|DamageActivation)
    (Utilities|FlowControl|Delay 2.5)
    (Variables|Default|SetSergentAttack false)
    (Development|PrintString " ATT END" true true "(R=0.222582,G=1.000000,B=0.000000,A=1.000000)")))

(fn ConstructionScript
  (|CallParentFunction))

(fn DeathRagdoll
  (Audio|PlaySoundatLocation "/Game/Ennemies/NPC/Sergent_2/Sergent_Death.Sergent_Death" (Transformation|GetActorLocation) "0, 0, 0" 1.0 1.0 0.0 0 0 0)
  (Physics|SetSimulatePhysics (Variables|Character|GetMesh) true)
  (Collision|SetCollisionEnabled (Variables|Default|GetCapsuleComponent) "QueryAndPhysics")
  (Collision|SetCollisionEnabled (Variables|Default|GetS_Spear-Primitive_1) "NoCollision")
  (Pawn|Components|CharacterMovement|DisableMovement (Variables|Character|GetCharacterMovement))
  (Components|Activation|Deactivate (Variables|Default|GetBlackboard)))