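; BP_Fishman_02 is a Grunt enemy NPC Blueprint that plays an attack montage on MeleeAttack and destroys itself when NPv drops to zero or below.
; NPv is checked every Tick, with no death animation played before destruction.
; The death montage, random NavMesh wandering, and perception logic are disconnected and never run, leaving their events and the sword overlap event empty.
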(event OnComponentBeginOverlap(S_Sword-Goblin_1)
  (params (OverlappedComponent :type Primitive%20Component%20Object%20Reference) (OtherActor :type Actor%20Object%20Reference) (OtherComp :type Primitive%20Component%20Object%20Reference) (OtherBodyIndex :type Integer) (bFromSweep :type Boolean) (SweepResult :type Hit%20Result%20Structure%20%28by%20ref%29)))

(event OnTargetPerceptionUpdated(AIPerception)
  (params (Actor :type Actor%20Object%20Reference) (Stimulus :type AI%20Stimulus%20Structure)))

(event Custom|MoveNPC
  ;[1 1 1] Déplacement aléatoire sur NavMesh
)

(event EventBeginPlay
  ;[1 1 1] Déplacement aléatoire sur NavMesh
)

(event Collision|EventActorBeginOverlap
  (params (OtherActor :type Actor%20Object%20Reference)))

(event EventTick
  (params (DeltaSeconds :type Float%20%28single-precision%29))
  (if (<= (Variables|Default|Getn_pv) 0.0)
    (Actor|DestroyActor)))

(event EventMeleeAttack
  ;[1 1 1] Animation d'attaque
  (Animation|Montage|PlayMontage (Variables|Character|GetMesh) "/Game/Ennemies/NPC/Grunt/Grunt_AttackMontage.Grunt_AttackMontage"))

(event EventGruntDeath
  ;[1 1 1] Animation de mort
)

(fn ConstructionScript
  (|CallParentFunction))